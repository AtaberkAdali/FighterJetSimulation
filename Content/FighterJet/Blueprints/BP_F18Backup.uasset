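; Player-controlled F-18 fighter jet pawn, named as a backup, that drives a vehicle movement component through Enhanced Input.
; Thrust and brake inputs ease a shared throttle value that feeds the movement component and HUD widget; handbrake, pitch and camera look are passed through directly.
; Each tick, that throttle scales both engines' Niagara exhaust and sets the jet engine sound's gain parameter.
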(event `self.ReceiveBeginPlay`
  (`EnhancedInputSubsystemInterface.AddMappingContext` (pcsubsystem `EnhancedInputLocalPlayerSubsystem` (`GameplayStatics.GetPlayerController` 0)) "/Game/FighterJet/Inputs/IMP_FighterJet.IMP_FighterJet" 0 (struct))
  (bind _returnvalue (`|CreateWidget` "/Game/FighterJet/Widgets/WBP_F18UI.WBP_F18UI_C"))
  (set `self.F18UI` _returnvalue)
  (`UserWidget.AddToViewport` _returnvalue 0))

(event `self.ReceiveTick`
  (params (DeltaSeconds :type "Float (single-precision)"))
  (`self.ManageThrottleVFX`))

(event `EnhancedInput|/Game/FighterJet/Inputs/IA_LookAround`
  (params (ActionValue :type "Vector2D Structure") (ElapsedSeconds :type "Float (double-precision)") (TriggeredSeconds :type "Float (double-precision)") (InputAction :type "InputAction Object Reference" :default "/Game/FighterJet/Inputs/IA_LookAround.IA_LookAround"))
  (:`Triggered`
    (`self.AddControllerYawInput` ActionValue_X)
    (`self.AddControllerPitchInput` ActionValue_Y)))

(event `EnhancedInput|/Game/FighterJet/Inputs/IA_Thrust`
  (params (ActionValue :type "Float (double-precision)") (ElapsedSeconds :type "Float (double-precision)") (TriggeredSeconds :type "Float (double-precision)") (InputAction :type "InputAction Object Reference" :default "/Game/FighterJet/Inputs/IA_Thrust.IA_Thrust"))
  (:`Triggered`
    (bind _output_get (set `self.throttleValue` (`KismetMathLibrary.FInterpTo` (`self.throttleValue`) ActionValue (`GameplayStatics.GetWorldDeltaSeconds`) 0.5)))
    (`/Game/FighterJet/Widgets/WBP_F18UI.SetThrottleImage` (`self.F18UI`) _output_get)
    (`ChaosVehicleMovementComponent.SetThrottleInput` (`self.VehicleMovementComponent`) _output_get)))

(event `EnhancedInput|/Game/FighterJet/Inputs/IA_Brake`
  (params (ActionValue :type "Float (double-precision)") (ElapsedSeconds :type "Float (double-precision)") (TriggeredSeconds :type "Float (double-precision)") (InputAction :type "InputAction Object Reference" :default "/Game/FighterJet/Inputs/IA_Brake.IA_Brake"))
  (:`Triggered`
    (bind _output_get (set `self.throttleValue` (`KismetMathLibrary.FInterpTo` (`self.throttleValue`) 0.0 (`GameplayStatics.GetWorldDeltaSeconds`) 0.5)))
    (`/Game/FighterJet/Widgets/WBP_F18UI.SetThrottleImage` (`self.F18UI`) _output_get)
    (`ChaosVehicleMovementComponent.SetThrottleInput` (`self.VehicleMovementComponent`) _output_get)))

(event `EnhancedInput|/Game/FighterJet/Inputs/IA_Handbrake`
  (params (ActionValue :type Boolean) (ElapsedSeconds :type "Float (double-precision)") (TriggeredSeconds :type "Float (double-precision)") (InputAction :type "InputAction Object Reference" :default "/Game/FighterJet/Inputs/IA_Handbrake.IA_Handbrake"))
  (bind _vehiclemovementcomponent (`self.VehicleMovementComponent`))
  (:`Started`
    (`ChaosVehicleMovementComponent.SetHandbrakeInput` _vehiclemovementcomponent true))
  (:`Completed`
    (`ChaosVehicleMovementComponent.SetHandbrakeInput` _vehiclemovementcomponent false)))

(event `EnhancedInput|/Game/FighterJet/Inputs/IA_Pitch`
  (params (ActionValue :type "Float (double-precision)") (ElapsedSeconds :type "Float (double-precision)") (TriggeredSeconds :type "Float (double-precision)") (InputAction :type "InputAction Object Reference" :default "/Game/FighterJet/Inputs/IA_Pitch.IA_Pitch"))
  (bind _vehiclemovementcomponent (`self.VehicleMovementComponent`))
  (:`Triggered`
    (`ChaosVehicleMovementComponent.SetPitchInput` _vehiclemovementcomponent ActionValue))
  (:`Completed`
    (`ChaosVehicleMovementComponent.SetPitchInput` _vehiclemovementcomponent 0.0)))

(fn `ManageThrottleVFX`
  (`FXSystemComponent.SetVectorParameter` (`self.RightEngineNiagara`) "Scale" (`KismetMathLibrary.MakeVector` (`self.throttleValue`) 1.0 1.0))
  (`FXSystemComponent.SetVectorParameter` (`self.LeftEngineNiagara`) "Scale" (`KismetMathLibrary.MakeVector` (`self.throttleValue`) 1.0 1.0))
  (`AudioComponent.SetFloatParameter` (`self.MS_JetEngine`) "Gain" (+ (`self.throttleValue`) 0.01)))

(fn `UserConstructionScript`)