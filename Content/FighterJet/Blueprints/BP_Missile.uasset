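; BP_Missile is a fighter jet missile projectile that homes in on an assigned target and explodes when it stops.
; On BeginPlay, a valid MTarget supplies a scene component as the ProjectileMovement homing target.
; When the projectile stops, it spawns a Niagara dust explosion and grenade sound at the impact location, then destroys itself.
; Tick accumulates delta time into MissileRotation, which nothing in these graphs reads.
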(event `self.ReceiveBeginPlay`
  (bind _mtarget (`self.MTarget`))
  (`/Engine/EditorBlueprintResources/StandardMacros.IsValid` _mtarget
    (:`Is Valid`
      (set `ProjectileMovementComponent.HomingTargetComponent` (`self.GetComponentByClass` _mtarget "/Script/Engine.SceneComponent") (`self.ProjectileMovement`)))))

(event `self.ReceiveTick`
  (params (DeltaSeconds :type "Float (single-precision)"))
  (set `self.MissileRotation` (+ (`self.MissileRotation`) DeltaSeconds)))

(event `self.ProjectileMovement.OnProjectileStop`
  (params (ImpactResult :type "HitResult Structure (by ref)"))
  (bind (_bblockinghit _binitialoverlap _time _distance _location) (`GameplayStatics.BreakHitResult` ImpactResult))
  (`NiagaraFunctionLibrary.SpawnSystemAtLocation` "/Game/FighterJet/Assets/VFX/Prefabs/Niagara_Dust_Explosion_01.Niagara_Dust_Explosion_01" _location)
  (`GameplayStatics.SpawnSoundAtLocation` "/Game/FighterJet/Assets/Sounds/ES_Grenade_Explosion_14_-_SFX_Producer.ES_Grenade_Explosion_14_-_SFX_Producer" _location (struct) 1.0 1.0 0.0 null null)
  (`self.K2_DestroyActor`))

(fn `UserConstructionScript`)