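; Player-flown F-18 jet pawn with target lock, missiles, retractable landing gear and a HUD.
; Enhanced Input is interpolated into the vehicle movement component, with timelines recentering axes; throttle also drives engine VFX and audio.
; A box picks "Target"-tagged actors for a marker and four timer-reloaded missiles, with the camera following each shot until fire is released.
; Any damage or excessive computed G-force destroys the jet and reloads GameMap after a delay.
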(event `ChangeTarget` :!signature `self.OnDestroyed`
  (params (DestroyedActor :type "Actor Object Reference"))
  ; Targeting SYstem
  (for _array_element (`PrimitiveComponent.GetOverlappingActors` (`self.Box`) null)
    (if (`self.ActorHasTag` _array_element "Target")
      (if (!= _array_element (`self.MyTarget`))
        (set `self.MyTarget` _array_element)
        (break)))))

(event `self.ReceiveAnyDamage`
  (params (Damage :type "Float (single-precision)") (DamageType :type "DamageType Object Reference") (InstigatedBy :type "Controller Object Reference") (DamageCauser :type "Actor Object Reference"))
  ; DESTROY THE F18
  (set `self.JetDestroyed` true :!label _label)
  (`NiagaraFunctionLibrary.SpawnSystemAtLocation` "/Game/FighterJet/Assets/VFX/Prefabs/Niagara_Dust_Explosion_01.Niagara_Dust_Explosion_01" (`self.K2_GetActorLocation`))
  (`GameplayStatics.SpawnSoundAtLocation` "/Game/FighterJet/Assets/Sounds/ES_Grenade_Explosion_14_-_SFX_Producer.ES_Grenade_Explosion_14_-_SFX_Producer" (`self.K2_GetActorLocation`) (struct) 1.0 1.0 0.0 null null)
  (`SceneComponent.SetVisibility` (`self.RightEngineNiagara`) false false)
  (`SceneComponent.SetVisibility` (`self.LeftEngineNiagara`) false false)
  (`AudioComponent.SetVolumeMultiplier` (`self.MS_JetEngine`) 0.0)
  (`MovementComponent.StopMovementImmediately` (`self.VehicleMovementComponent`))
  (`PrimitiveComponent.SetMaterial` (`self.Mesh`) 0 "/Game/FighterJet/Assets/Meshes/West_Fighter_F18C/Damaged/Materials/M_West_Fighter_F18C_Damaged.M_West_Fighter_F18C_Damaged")
  (`SceneComponent.SetVisibility` (`self.Missile02`) false false)
  (`SceneComponent.SetVisibility` (`self.Missile03`) false false)
  (`SceneComponent.SetVisibility` (`self.Missile04`) false false)
  (`SceneComponent.SetVisibility` (`self.Missile01`) false false)
  (`KismetSystemLibrary.K2_SetTimerDelegate` (delegate `RestartGame`) 3.0))

(event `self.ReceiveTick`
  (params (DeltaSeconds :type "Float (single-precision)"))
  (bind _widgetbp (`self.WidgetBP`))
  (bind _returnvalue (`KismetMathLibrary.Abs` (`self.GForce`)))
  (if (not (`self.JetDestroyed`))
    (`self.ManageThrottleVFX`)
    (`|ExecutionSequence`
      (:`then_0`
        ; Targeting SYstem
        (`/Engine/EditorBlueprintResources/StandardMacros.IsValid` (`self.MyTarget`)
          (:`Is Valid`
            (`SceneComponent.K2_SetWorldLocation` _widgetbp (`self.K2_GetActorLocation` (`self.MyTarget`)) false false)
            (`SceneComponent.SetVisibility` _widgetbp true false)
            (add `self.OnDestroyed` (`self.MyTarget`) (delegate `ChangeTarget`)))
          (:`Is Not Valid`
            (`SceneComponent.SetVisibility` (`self.WidgetBP`) false false))))
      (:`then_1`
        (set `self.CurrentFrameVelocity` (`KismetMathLibrary.VSize` (`self.GetVelocity`)))
        ; Calculate GForce Velocity
        (set `self.GForce` (/ (- (`self.CurrentFrameVelocity`) (`self.LastFrameVelocity_0`)) (* (`GameplayStatics.GetWorldDeltaSeconds`) (`MovementComponent.GetGravityZ` (`self.VehicleMovementComponent`)))))
        (set `self.LastFrameVelocity_0` (`KismetMathLibrary.VSize` (`self.GetVelocity`)))
        (if (> _returnvalue 10.0)
          (`KismetSystemLibrary.PrintString` (`KismetStringLibrary.Concat_StrStr` "Crush GForce: " (`KismetStringLibrary.Conv_DoubleToString` _returnvalue)) true true (struct :`R` 1.0 :`B` 0.15978 :`A` 1.0) 10.0)
          (goto _label))))))

(event `RestartGame`
  (`GameplayStatics.OpenLevel` "GameMap"))

(event `self.ReceiveBeginPlay`
  (`EnhancedInputSubsystemInterface.AddMappingContext` (pcsubsystem `EnhancedInputLocalPlayerSubsystem` (`GameplayStatics.GetPlayerController` 0)) "/Game/FighterJet/Inputs/IMP_FighterJet.IMP_FighterJet" 0 (struct))
  (bind _returnvalue (`|CreateWidget` "/Game/FighterJet/Widgets/WBP_F18UI.WBP_F18UI_C"))
  (set `self.F18UI` _returnvalue)
  (`UserWidget.AddToViewport` _returnvalue 0))

(event `EnhancedInput|/Game/FighterJet/Inputs/IA_LookAround`
  (params (ActionValue :type "Vector2D Structure") (ElapsedSeconds :type "Float (double-precision)") (TriggeredSeconds :type "Float (double-precision)") (InputAction :type "InputAction Object Reference" :default "/Game/FighterJet/Inputs/IA_LookAround.IA_LookAround"))
  (:`Triggered`
    (`self.AddControllerYawInput` ActionValue_X)
    (`self.AddControllerPitchInput` ActionValue_Y)))

(event `EnhancedInput|/Game/FighterJet/Inputs/IA_Thrust`
  (params (ActionValue :type "Float (double-precision)") (ElapsedSeconds :type "Float (double-precision)") (TriggeredSeconds :type "Float (double-precision)") (InputAction :type "InputAction Object Reference" :default "/Game/FighterJet/Inputs/IA_Thrust.IA_Thrust"))
  (:`Triggered`
    (if (not (`self.JetDestroyed`))
      (bind _output_get (set `self.throttleValue` (`KismetMathLibrary.FInterpTo` (`self.throttleValue`) ActionValue (`GameplayStatics.GetWorldDeltaSeconds`) 0.5)))
      (`/Game/FighterJet/Widgets/WBP_F18UI.SetThrottleImage` (`self.F18UI`) _output_get)
      (`ChaosVehicleMovementComponent.SetThrottleInput` (`self.VehicleMovementComponent`) _output_get))))

(event `EnhancedInput|/Game/FighterJet/Inputs/IA_Brake`
  (params (ActionValue :type "Float (double-precision)") (ElapsedSeconds :type "Float (double-precision)") (TriggeredSeconds :type "Float (double-precision)") (InputAction :type "InputAction Object Reference" :default "/Game/FighterJet/Inputs/IA_Brake.IA_Brake"))
  (:`Triggered`
    (if (not (`self.JetDestroyed`))
      (bind _output_get (set `self.throttleValue` (`KismetMathLibrary.FInterpTo` (`self.throttleValue`) 0.0 (`GameplayStatics.GetWorldDeltaSeconds`) 0.5)))
      (`/Game/FighterJet/Widgets/WBP_F18UI.SetThrottleImage` (`self.F18UI`) _output_get)
      (`ChaosVehicleMovementComponent.SetThrottleInput` (`self.VehicleMovementComponent`) _output_get))))

(event `EnhancedInput|/Game/FighterJet/Inputs/IA_Handbrake`
  (params (ActionValue :type Boolean) (ElapsedSeconds :type "Float (double-precision)") (TriggeredSeconds :type "Float (double-precision)") (InputAction :type "InputAction Object Reference" :default "/Game/FighterJet/Inputs/IA_Handbrake.IA_Handbrake"))
  (bind _vehiclemovementcomponent (`self.VehicleMovementComponent`))
  (:`Started`
    (if (not (`self.JetDestroyed`))
      (`ChaosVehicleMovementComponent.SetHandbrakeInput` _vehiclemovementcomponent true)))
  (:`Completed`
    (`ChaosVehicleMovementComponent.SetHandbrakeInput` _vehiclemovementcomponent false)))

(event `EnhancedInput|/Game/FighterJet/Inputs/IA_Pitch`
  (params (ActionValue :type "Float (double-precision)") (ElapsedSeconds :type "Float (double-precision)") (TriggeredSeconds :type "Float (double-precision)") (InputAction :type "InputAction Object Reference" :default "/Game/FighterJet/Inputs/IA_Pitch.IA_Pitch"))
  (bind _vehiclemovementcomponent (`self.VehicleMovementComponent`))
  (bind _returnvalue (`KismetMathLibrary.FInterpTo` (`self.PitchValue`) ActionValue (`GameplayStatics.GetWorldDeltaSeconds`) 5.0))
  (:`Triggered`
    (if (not (`self.JetDestroyed`))
      (set `self.PitchValue` _returnvalue)
      (`ChaosVehicleMovementComponent.SetPitchInput` _vehiclemovementcomponent (* _returnvalue -1.0))))
  (:`Started`
    (`Timeline|PitchToZero` :!via `Stop` :!label _label_2
      (:`Update`
        (bind _output_get (set `self.PitchValue` (`KismetMathLibrary.FInterpTo` (`self.PitchValue`) 0.0 (`GameplayStatics.GetWorldDeltaSeconds`) 5.0)))
        (`ChaosVehicleMovementComponent.SetPitchInput` _vehiclemovementcomponent _output_get))))
  (:`Completed`
    (goto _label_2 :!via `PlayFromStart`)))

(event `EnhancedInput|/Game/FighterJet/Inputs/IA_Roll`
  (params (ActionValue :type "Float (double-precision)") (ElapsedSeconds :type "Float (double-precision)") (TriggeredSeconds :type "Float (double-precision)") (InputAction :type "InputAction Object Reference" :default "/Game/FighterJet/Inputs/IA_Roll.IA_Roll"))
  (bind _vehiclemovementcomponent (`self.VehicleMovementComponent`))
  (:`Triggered`
    (if (not (`self.JetDestroyed`))
      (bind _output_get (set `self.RollValue` (`KismetMathLibrary.FInterpTo` (`self.RollValue`) ActionValue (`GameplayStatics.GetWorldDeltaSeconds`) 5.0)))
      (`ChaosVehicleMovementComponent.SetRollInput` _vehiclemovementcomponent _output_get)))
  (:`Started`
    (`Timeline|RollTheZero` :!via `Stop` :!label _label_3
      (:`Update`
        (bind _output_get_2 (set `self.RollValue` (`KismetMathLibrary.FInterpTo` (`self.RollValue`) 0.0 (`GameplayStatics.GetWorldDeltaSeconds`) 5.0)))
        (`ChaosVehicleMovementComponent.SetRollInput` _vehiclemovementcomponent _output_get_2))))
  (:`Completed`
    (goto _label_3 :!via `PlayFromStart`)))

(event `EnhancedInput|/Game/FighterJet/Inputs/IA_Yaw`
  (params (ActionValue :type "Float (double-precision)") (ElapsedSeconds :type "Float (double-precision)") (TriggeredSeconds :type "Float (double-precision)") (InputAction :type "InputAction Object Reference" :default "/Game/FighterJet/Inputs/IA_Yaw.IA_Yaw"))
  (bind _vehiclemovementcomponent (`self.VehicleMovementComponent`))
  (:`Triggered`
    (if (not (`self.JetDestroyed`))
      (bind _output_get (set `self.YawValue` (`KismetMathLibrary.FInterpTo` (`self.YawValue`) ActionValue (`GameplayStatics.GetWorldDeltaSeconds`) 5.0)))
      (`ChaosVehicleMovementComponent.SetYawInput` _vehiclemovementcomponent _output_get)))
  (:`Started`
    (`Timeline|YawToZero` :!via `Stop` :!label _label_4
      (:`Update`
        (bind _output_get_2 (set `self.YawValue` (`KismetMathLibrary.FInterpTo` (`self.YawValue`) 0.0 (`GameplayStatics.GetWorldDeltaSeconds`) 5.0)))
        (`ChaosVehicleMovementComponent.SetYawInput` _vehiclemovementcomponent _output_get_2))))
  (:`Completed`
    (goto _label_4 :!via `PlayFromStart`)))

(event `EnhancedInput|/Game/FighterJet/Inputs/IA_Gear`
  (params (ActionValue :type Boolean) (ElapsedSeconds :type "Float (double-precision)") (TriggeredSeconds :type "Float (double-precision)") (InputAction :type "InputAction Object Reference" :default "/Game/FighterJet/Inputs/IA_Gear.IA_Gear"))
  (:`Started`
    (if (`self.JetDestroyed`)
      _
      (elif (`self.IsGearOpen?`)
        (bind _isinair (`self.CheckAltitude`))
        (if _isinair
          (bind (_direction _gears _gearsdoor) (`Timeline|GearsTimeline` :!label _label_5)
            (:`Update`
              (set `self.Gears` _gears)
              (set `self.Gears Door` _gearsdoor))
            (:`Finished`
              (set `self.IsGearOpen?` (not (`self.IsGearOpen?`))))))
        (else
          (goto _label_5 :!via `Reverse`))))))

(event `EnhancedInput|/Game/FighterJet/Inputs/IA_Fire1`
  (params (ActionValue :type Boolean) (ElapsedSeconds :type "Float (double-precision)") (TriggeredSeconds :type "Float (double-precision)") (InputAction :type "InputAction Object Reference" :default "/Game/FighterJet/Inputs/IA_Fire1.IA_Fire1"))
  (bind _missile01 (`self.Missile01`))
  (bind _missile02 (`self.Missile02`))
  (bind _missile03 (`self.Missile03`))
  (bind _missile04 (`self.Missile04`))
  (:`Started`
    (if (`self.JetDestroyed`)
      _
      (elif (`SceneComponent.bVisible` (`self.Missile01`))
        (`KismetSystemLibrary.PrintString` "missile 1 fired")
        (`SceneComponent.SetVisibility` _missile01 false false)
        (`/Game/FighterJet/Widgets/WBP_F18UI.SetMissileUIVisibility` (`self.F18UI`) 1 false)
        (bind _returnvalue (`|SpawnActorFromClass` "/Game/FighterJet/Blueprints/BP_Missile.BP_Missile_C" (`SceneComponent.K2_GetComponentToWorld` _missile01) "AdjustIfPossibleButAlwaysSpawn" "MultiplyWithRoot" null (`self.MyTarget`) null))
        (`PlayerController.SetViewTargetWithBlend` (`GameplayStatics.GetPlayerController` 0) _returnvalue 2.0 "VTBlend_EaseInOut" 5.0 false)
        (`KismetSystemLibrary.K2_SetTimerDelegate` (delegate `Missile1Event`) (`self.ReloadTime`))
        (elif (`SceneComponent.bVisible` (`self.Missile02`))
          (`KismetSystemLibrary.PrintString` "missile 2 fired")
          (`SceneComponent.SetVisibility` _missile02 false false)
          (`/Game/FighterJet/Widgets/WBP_F18UI.SetMissileUIVisibility` (`self.F18UI`) 2 false)
          (bind _returnvalue_2 (`|SpawnActorFromClass` "/Game/FighterJet/Blueprints/BP_Missile.BP_Missile_C" (`SceneComponent.K2_GetComponentToWorld` _missile02) "AdjustIfPossibleButAlwaysSpawn" "MultiplyWithRoot" null (`self.MyTarget`) null))
          (`PlayerController.SetViewTargetWithBlend` (`GameplayStatics.GetPlayerController` 0) _returnvalue_2 2.0 "VTBlend_EaseInOut" 5.0 false)
          (`KismetSystemLibrary.K2_SetTimerDelegate` (delegate `Misile2`) (`self.ReloadTime`))
          (elif (`SceneComponent.bVisible` (`self.Missile03`))
            (`KismetSystemLibrary.PrintString` "missile 3 fired")
            (`SceneComponent.SetVisibility` _missile03 false false)
            (`/Game/FighterJet/Widgets/WBP_F18UI.SetMissileUIVisibility` (`self.F18UI`) 3 false)
            (bind _returnvalue_3 (`|SpawnActorFromClass` "/Game/FighterJet/Blueprints/BP_Missile.BP_Missile_C" (`SceneComponent.K2_GetComponentToWorld` _missile03) "AdjustIfPossibleButAlwaysSpawn" "MultiplyWithRoot" null (`self.MyTarget`) null))
            (`PlayerController.SetViewTargetWithBlend` (`GameplayStatics.GetPlayerController` 0) _returnvalue_3 2.0 "VTBlend_EaseInOut" 5.0 false)
            (`KismetSystemLibrary.K2_SetTimerDelegate` (delegate `Misile3`) (`self.ReloadTime`))
            (elif (`SceneComponent.bVisible` (`self.Missile04`))
              (`KismetSystemLibrary.PrintString` "missile 4 fired")
              (`SceneComponent.SetVisibility` _missile04 false false)
              (`/Game/FighterJet/Widgets/WBP_F18UI.SetMissileUIVisibility` (`self.F18UI`) 4 false)
              (bind _returnvalue_4 (`|SpawnActorFromClass` "/Game/FighterJet/Blueprints/BP_Missile.BP_Missile_C" (`SceneComponent.K2_GetComponentToWorld` _missile04) "AdjustIfPossibleButAlwaysSpawn" "MultiplyWithRoot" null (`self.MyTarget`) null))
              (`PlayerController.SetViewTargetWithBlend` (`GameplayStatics.GetPlayerController` 0) _returnvalue_4 2.0 "VTBlend_EaseInOut" 5.0 false)
              (`KismetSystemLibrary.K2_SetTimerDelegate` (delegate `Misile4`) (`self.ReloadTime`))))))))
  (:`Completed`
    (`PlayerController.SetViewTargetWithBlend` (`GameplayStatics.GetPlayerController` 0) self 0.0 "VTBlend_EaseInOut" 5.0 false)))

(event `Missile1Event`
  (`SceneComponent.SetVisibility` (`self.Missile01`) true false)
  (`/Game/FighterJet/Widgets/WBP_F18UI.SetMissileUIVisibility` (`self.F18UI`) 1 true))

(event `Misile2`
  (`SceneComponent.SetVisibility` (`self.Missile02`) true false)
  (`/Game/FighterJet/Widgets/WBP_F18UI.SetMissileUIVisibility` (`self.F18UI`) 2 true))

(event `Misile3`
  (`SceneComponent.SetVisibility` (`self.Missile03`) true false)
  (`/Game/FighterJet/Widgets/WBP_F18UI.SetMissileUIVisibility` (`self.F18UI`) 3 true))

(event `Misile4`
  (`SceneComponent.SetVisibility` (`self.Missile04`) true false)
  (`/Game/FighterJet/Widgets/WBP_F18UI.SetMissileUIVisibility` (`self.F18UI`) 4 true))

(event `self.Box.OnComponentBeginOverlap`
  (params (OverlappedComponent :type "PrimitiveComponent Object Reference") (OtherActor :type "Actor Object Reference") (OtherComp :type "PrimitiveComponent Object Reference") (OtherBodyIndex :type Integer) (bFromSweep :type Boolean) (SweepResult :type "HitResult Structure (by ref)"))
  (if (`self.ActorHasTag` OtherActor "Target")
    (set `self.MyTarget` OtherActor)))

(event `EnhancedInput|/Game/FighterJet/Inputs/IA_ChangeTarget`
  (params (ActionValue :type Boolean) (ElapsedSeconds :type "Float (double-precision)") (TriggeredSeconds :type "Float (double-precision)") (InputAction :type "InputAction Object Reference" :default "/Game/FighterJet/Inputs/IA_ChangeTarget.IA_ChangeTarget"))
  (:`Started`
    (if (not (`self.JetDestroyed`))
      (`self.ChangeTarget` null))))

(fn `CheckAltitude`
  (returns (isInAir :type Boolean))
  (bind _returnvalue (`SceneComponent.K2_GetComponentLocation` (`self.SpringArm`)))
  (bind _outhit (`KismetSystemLibrary.LineTraceSingle` :`Start` _returnvalue :`End` (- _returnvalue (0.0 0.0 2000.0)) :`TraceChannel` "TraceTypeQuery1" :`DrawDebugType` "Persistent"))
  (bind (_bblockinghit _binitialoverlap _time _distance) (`GameplayStatics.BreakHitResult` _outhit))
  (if _bblockinghit
    (if (> _distance 250.0)
      _
      (else
        (return false))))
  (return true))

(fn `ManageThrottleVFX`
  (`FXSystemComponent.SetVectorParameter` (`self.RightEngineNiagara`) "Scale" (`KismetMathLibrary.MakeVector` (`self.throttleValue`) 1.0 1.0))
  (`FXSystemComponent.SetVectorParameter` (`self.LeftEngineNiagara`) "Scale" (`KismetMathLibrary.MakeVector` (`self.throttleValue`) 1.0 1.0))
  (`AudioComponent.SetFloatParameter` (`self.MS_JetEngine`) "Gain" (+ (`self.throttleValue`) 0.01)))

(fn `UserConstructionScript`)