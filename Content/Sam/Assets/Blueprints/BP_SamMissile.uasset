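; BP_SamMissile is a homing missile projectile that damages what it hits and explodes.
; On BeginPlay it feeds a scene component of MTarget, if valid, to ProjectileMovement as the homing target and starts a lifetime timer.
; When the projectile stops, it applies fixed damage to the hit actor, spawns explosion effects and sound, then destroys itself.
; When the timer expires, it explodes in place with the same effects but deals no damage.
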(event `self.ReceiveBeginPlay`
  (bind _mtarget (`self.MTarget`))
  (`|ExecutionSequence`
    (:`then_0`
      (`/Engine/EditorBlueprintResources/StandardMacros.IsValid` _mtarget
        (:`Is Valid`
          (set `ProjectileMovementComponent.HomingTargetComponent` (`self.GetComponentByClass` _mtarget "/Script/Engine.SceneComponent") (`self.ProjectileMovement`)))))
    (:`then_1`
      (`KismetSystemLibrary.K2_SetTimerDelegate` (delegate `Explode`) (`self.MissileLifeTime`)))))

(event `Explode`
  (bind _returnvalue (`self.K2_GetActorLocation`))
  (`NiagaraFunctionLibrary.SpawnSystemAtLocation` "/Game/FighterJet/Assets/VFX/Prefabs/Niagara_Dust_Explosion_01.Niagara_Dust_Explosion_01" _returnvalue)
  (`GameplayStatics.SpawnSoundAtLocation` "/Game/FighterJet/Assets/Sounds/ES_Grenade_Explosion_14_-_SFX_Producer.ES_Grenade_Explosion_14_-_SFX_Producer" _returnvalue (struct) 1.0 1.0 0.0 null null)
  (`self.K2_DestroyActor`))

(event `self.ProjectileMovement.OnProjectileStop`
  (params (ImpactResult :type "HitResult Structure (by ref)"))
  (bind (_bblockinghit _binitialoverlap _time _distance _location _impactpoint _normal _impactnormal _physmat _hitactor) (`GameplayStatics.BreakHitResult` ImpactResult))
  (`GameplayStatics.ApplyDamage` _hitactor 10.0)
  (`NiagaraFunctionLibrary.SpawnSystemAtLocation` "/Game/FighterJet/Assets/VFX/Prefabs/Niagara_Dust_Explosion_01.Niagara_Dust_Explosion_01" _location)
  (`GameplayStatics.SpawnSoundAtLocation` "/Game/FighterJet/Assets/Sounds/ES_Grenade_Explosion_14_-_SFX_Producer.ES_Grenade_Explosion_14_-_SFX_Producer" _location (struct) 1.0 1.0 0.0 null null)
  (`self.K2_DestroyActor`))

(fn `UserConstructionScript`)